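; BP_BaseInteractable is a base interactable that registers itself with the ThirdPersonCharacter while that character is inside its InteractableArea.
; Begin and end overlap send register and unregister calls to the character, passing itself.
; SetHighlight toggles custom depth rendering on InteractableMesh.
; The Interaction event only prints a debug string, and the Interact input runs a short delay with nothing after it.
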(event OnComponentBeginOverlap(InteractableArea)
  (params (OverlappedComponent :type Primitive%20Component%20Object%20Reference) (OtherActor :type Actor%20Object%20Reference) (OtherComp :type Primitive%20Component%20Object%20Reference) (OtherBodyIndex :type Integer) (bFromSweep :type Boolean) (SweepResult :type Hit%20Result%20Structure%20%28by%20ref%29))
  (bind _asthird_person_character (Utilities|Casting|CastToThirdPersonCharacter OtherActor))
  (Class|BPIInteract|RegisterInteractable(Message) _asthird_person_character self))

(event OnComponentEndOverlap(InteractableArea)
  (params (OverlappedComponent :type Primitive%20Component%20Object%20Reference) (OtherActor :type Actor%20Object%20Reference) (OtherComp :type Primitive%20Component%20Object%20Reference) (OtherBodyIndex :type Integer))
  (bind _asthird_person_character (Utilities|Casting|CastToThirdPersonCharacter OtherActor))
  (Class|BPIInteract|UnregisterInteractable(Message) _asthird_person_character self))

(event EventInteraction
  (params (Instigator :type Third%20Person%20Character%20Object%20Reference))
  (Development|PrintString "Recieved"))

(event Input|ActionEvents|InputActionInteract
  (params (Key :type Key%20Structure))
  (:Pressed
    (Utilities|FlowControl|Delay 0.2)))

(fn ConstructionScript)

(fn SetHighlight
  (params (Highlight :type Boolean))
  (Rendering|SetRenderCustomDepth (Variables|Default|GetInteractableMesh) Highlight))